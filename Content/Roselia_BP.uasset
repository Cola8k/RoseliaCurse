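; Roselia Blueprint that tracks a fear meter, likely for a game character, and puts a HUD on screen.
; BeginPlay creates the HUD_BP widget with a reference to itself and adds it to the viewport.
; FearPercentage returns Fear divided by FearMax, and Tick prints that ratio every frame as debug output.
; Nothing in these graphs changes the Fear value.
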(event EventBeginPlay
  (bind _returnvalue (UserInterface|CreateWidget "/Game/HUD_BP.HUD_BP_C" 0 self))
  (UserInterface|Viewport|AddtoViewport _returnvalue 0))

(event Collision|EventActorBeginOverlap
  (params (OtherActor :type Actor%20Object%20Reference)))

(event EventTick
  (params (DeltaSeconds :type Float%20%28single-precision%29))
  (Development|PrintString (Utilities|String|ToString(Float) (CallFunction|FearPercentage))))

(fn ConstructionScript)

(fn FearPercentage
  (return (/ (Variables|Default|GetFear) (Variables|Default|GetFearMax))))