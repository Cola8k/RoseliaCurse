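; Door actor that raises and lowers its cube mesh and acts as a trigger for changing rooms.
; OpenDoor and CloseDoor play and reverse a timeline that offsets the cube's Z from its start location cached on BeginPlay.
; When a component tagged PlayerBody overlaps the box, it finds GM_BP and calls ChangeRoom with the SpawnPointPlayer world location.
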(event OnComponentBeginOverlap(Box)
  (params (OverlappedComponent :type Primitive%20Component%20Object%20Reference) (OtherActor :type Actor%20Object%20Reference) (OtherComp :type Primitive%20Component%20Object%20Reference) (OtherBodyIndex :type Integer) (bFromSweep :type Boolean) (SweepResult :type Hit%20Result%20Structure%20%28by%20ref%29))
  (if (Components|ComponentHasTag OtherComp "PlayerBody")
    (bind _returnvalue (Actor|GetActorOfClass "/Game/GM_BP.GM_BP_C"))
    (Default|ChangeRoom _returnvalue (Transformation|GetWorldLocation (Variables|Default|GetSpawnPointPlayer)))))

(event Custom|OpenDoor
  (bind _doorstartlocation (Variables|Default|GetDoorStartLocation))
  (bind _newtrack_0 (Timeline|OpenDoor_TM Play)
    (:Update
      (Transformation|SetWorldLocation (Variables|Default|GetCube) (Math|Vector|MakeVector (.x _doorstartlocation) (.y _doorstartlocation) (+ (.z _doorstartlocation) _newtrack_0)) false false))))

(event Custom|CloseDoor
  (bind _doorstartlocation (Variables|Default|GetDoorStartLocation))
  (bind _newtrack_0 (Timeline|OpenDoor_TM Reverse)
    (:Update
      (Transformation|SetWorldLocation (Variables|Default|GetCube) (Math|Vector|MakeVector (.x _doorstartlocation) (.y _doorstartlocation) (+ (.z _doorstartlocation) _newtrack_0)) false false))))

(event EventBeginPlay
  (Variables|Default|SetDoorStartLocation (Transformation|GetWorldLocation (Variables|Default|GetCube))))

(fn ConstructionScript)