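; Bomb enemy Blueprint that turns into a kamikaze charger when its FearSwitch event fires.
; FearSwitch clears a stored timer, stops the AI brain logic and snaps rotation once toward the Roselia_BP actor.
; The Kamikaze timeline then teleports it along its forward vector without sweep or homing, stepping by the track value each update.
; When the timeline finishes, a short life span destroys the enemy.
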(event EventBeginPlay)

(event Collision|EventActorBeginOverlap
  (params (OtherActor :type Actor%20Object%20Reference)))

(event EventTick
  (params (DeltaSeconds :type Float%20%28single-precision%29)))

(event EventFearSwitch
  (Utilities|Time|ClearandInvalidateTimerbyHandle (Variables|Default|GetTimerHandleRef))
  (AI|Logic|StopLogic (Variables|/Script/AIModule.AIController|GetBrainComponent (Variables|Default|GetAIController)) "")
  (bind _returnvalue (Actor|GetActorOfClass "/Game/Roselia_BP.Roselia_BP_C"))
  (Transformation|SetActorRotation (Math|Rotator|FindLookatRotation (Transformation|GetActorLocation) (Transformation|GetActorLocation _returnvalue)) true)
  (bind _lenght (Timeline|Kamikaze Play)
    (:Update
      (Transformation|SetActorLocation (+ (Transformation|GetActorLocation) (* (Transformation|GetActorForwardVector) _lenght)) false true))
    (:Finished
      (Actor|SetLifeSpan 0.1))))

(fn ConstructionScript)