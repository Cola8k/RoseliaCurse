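; Blueprint for a simple enemy that can be frightened by the Roselia actor.
; Shortly after BeginPlay it finds Roselia and binds FearSwitch to its fear delegate.
; FearSwitch sets the bIsScared blackboard key true and starts a four-second timer, after which CheckScared clears it for the AI to read.
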(event Custom|CheckScared
  (bind _output_get (Variables|Default|SetbIsFeared false))
  (AI|Components|Blackboard|SetValueasBool (AI|GetBlackboard self) (Utilities|Name|MakeLiteralName "bIsScared") _output_get))

(event Collision|EventActorBeginOverlap
  (params (OtherActor :type Actor%20Object%20Reference)))

(event EventTick
  (params (DeltaSeconds :type Float%20%28single-precision%29)))

(event EventBeginPlay
  (Utilities|FlowControl|Delay 0.2)
  (bind _returnvalue (Actor|GetActorOfClass "/Script/RoseliaCurse.Roselia"))
  (EventDispatchers|BindEventtoFearDelegate _returnvalue (delegate EventFearSwitch)))

(event EventFearSwitch
  (bind _output_get (Variables|Default|SetbIsFeared true))
  (AI|Components|Blackboard|SetValueasBool (AI|GetBlackboard self) (Utilities|Name|MakeLiteralName "bIsScared") _output_get)
  (Utilities|Time|SetTimerbyEvent (delegate Custom|CheckScared) 4.0))

(fn ConstructionScript)