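; GM_BP, apparently a game mode, holds logic for spawning a boss fight, but its SpawnBoss event is empty.
; A disconnected chain stores TentacleSP marker transforms and the BossSP marker transform.
; That chain would spawn a Tentacle at each stored transform, printing each one, and a BossEnemy at the boss point.
; As wired, none of this spawning logic runs.
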(event EventSpawnBoss)

(fn ConstructionScript)